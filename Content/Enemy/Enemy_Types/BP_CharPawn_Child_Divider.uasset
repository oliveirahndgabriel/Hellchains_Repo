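; Enemy pawn child of a shared CharPawn base that splits into two smaller Divider Mini enemies when it dies.
; On BeginPlay it runs the parent logic and binds SpawnDivider to the Mortis event.
; SpawnDivider checks IsDead, then spawns the two minis at the mesh location, offset to opposite sides along world Y.
; A HasDivide flag keeps the split from happening more than once.
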(event Custom|SpawnDivider
  (bind _mesh (Variables|Character|GetMesh))
  (bind _mesh_2 (Variables|Character|GetMesh))
  (if (Variables|Default|GetIsDead)
    (if (not (Variables|Default|GetHasDivide))
      (Game|SpawnActorfromClass "/Game/Enemy/Enemy_Types/BP_CharPawn_Child_DividerMini.BP_CharPawn_Child_DividerMini_C" (Math|Transform|MakeTransform (+ (Transformation|GetWorldLocation _mesh) "0.000000,80.000000,0.000000") (Transformation|GetWorldRotation _mesh) "1.000000,1.000000,1.000000") "AdjustIfPossibleButAlwaysSpawn" "MultiplyWithRoot" 0 0)
      (Game|SpawnActorfromClass "/Game/Enemy/Enemy_Types/BP_CharPawn_Child_DividerMini.BP_CharPawn_Child_DividerMini_C" (Math|Transform|MakeTransform (+ (Transformation|GetWorldLocation _mesh_2) "0.000000,-80.000000,0.000000") (Transformation|GetWorldRotation _mesh_2) "1.000000,1.000000,1.000000") "AdjustIfPossibleButAlwaysSpawn" "MultiplyWithRoot" 0 0)
      (Variables|Default|SetHasDivide true))))

(event EventBeginPlay
  (|CallParentFunction)
  (EventDispatchers|BindEventtoMortis (delegate Custom|SpawnDivider)))

(event Collision|EventActorBeginOverlap
  (params (OtherActor :type Actor%20Object%20Reference)))

(event EventTick
  (params (DeltaSeconds :type Float%20%28single-precision%29))
  (|CallParentFunction DeltaSeconds))

(fn ConstructionScript
  (|CallParentFunction))