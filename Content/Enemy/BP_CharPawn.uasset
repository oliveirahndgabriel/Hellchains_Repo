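; BP_CharPawn is an enemy character that takes damage from the first-person player's chain attack and dies at zero health.
; DamagePawn subtracts the player's current chain damage, while Knockback stops movement and applies a fixed world-X velocity impulse.
; Tick polls health and, once, enables player recovery, spawns BP_SoulsOfPain, flags death, then calls CallMortis and destroys itself after a delay.
; Camera-facing sight bar rotation is present but never runs.
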(event EventBeginPlay
  ;[1 1 1] Event Begin - Set Up Stuff
  (bind _output_get (Variables|Default|SetHealthCurrent (Variables|Default|GetHealthMax)))
  (Development|PrintString (Utilities|String|ToString(Float) _output_get))
  (bind _returnvalue (Actor|GetActorOfClass "/Game/FirstPerson/Blueprints/BP_FirstPersonCharacter.BP_FirstPersonCharacter_C"))
  (Variables|Default|SetPlayer _returnvalue))

(event EventTick
  (params (DeltaSeconds :type Float%20%28single-precision%29))
  (bind _player (Variables|Default|GetPlayer))
  ;[1 1 1] Event Tick
  (if (<= (Variables|Default|GetHealthCurrent) 0.0)
    (Utilities|FlowControl|DoOnce false
      (:Completed
        (Variables|/Game/FirstPerson/Blueprints/BP_FirstPersonCharacter.BP_FirstPersonCharacter_C|SetCanRecover _player true)
        (Class|BPIDamageInterface|CheckRecover(Message) _player)
        (Game|SpawnActorfromClass "/Game/Items/BP_SoulsOfPain.BP_SoulsOfPain_C" (Transformation|GetActorTransform) "AlwaysSpawn" "MultiplyWithRoot" 0 0)
        (Variables|Default|SetIsDead true)
        (Utilities|FlowControl|Delay 0.5)
        (Default|CallMortis)
        (Actor|DestroyActor)))))

(event EventKnockback
  (params (NewParam :type Vector :default "0, 0, 0"))
  ;[1 1 1] Event Interface - Add Impulse for knockback after being hitted
  (Class|NavMovementComponent|StopActiveMovement (Variables|Character|GetCharacterMovement))
  (Physics|AddImpulse (Variables|Character|GetCharacterMovement) "2000.000000,0.000000,0.000000" true))

(event EventDamagePawn
  ;[1 1 1] Event Receive Damage
  (bind _output_get (Variables|Default|SetHealthCurrent (- (Variables|Default|GetHealthCurrent) (Variables|/Game/FirstPerson/Blueprints/BP_FirstPersonCharacter.BP_FirstPersonCharacter_C|GetChainDamage_Current (Variables|Default|GetPlayer)))))
  (Development|PrintString (Utilities|String|ToString(Float) _output_get)))

(fn ConstructionScript)