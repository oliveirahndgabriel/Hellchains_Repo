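; Enemy AI controller that runs BT_Enemy and turns perception updates into Blackboard values for chasing.
; Successful sight sets TargetActor and sends a start-chase message; other updates send stop-chase and, if CanChase is false, store the actor's location and clear the target.
; StartChase sets CanChase, while StopChase clears it after a retriggerable five-second delay.
; A hearing handler that stores the stimulus location exists but is never called here.
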(event OnTargetPerceptionUpdated(AIPerception)
  (params (Actor :type Actor%20Object%20Reference) (Stimulus :type AI%20Stimulus%20Structure))
  ;[1 1 1] AI Perception (Target Updated) - Check AI Perception for Sight and Sound
  (CallFunction|HandleSightPerception Actor Stimulus))

(event Custom|Detection%20Update
  (params (Bool :type %20Object%20Reference) (Actor :type Actor%20Object%20Reference))
  ;[1 1 1] Custom Event - Handle Start & Stop Detection
)

(event EventBeginPlay
  ;[1 1 1] Event BeginPlay - Start Behavior Tree and set Controlled Pawn
  (AI|RunBehaviorTree "/Game/Enemy/BT_Enemy.BT_Enemy")
  (Variables|Default|SetControlledPawn (Pawn|GetControlledPawn)))

(event EventStartChase
  ;[1 1 1] Start & Stop Chase Event - Set Blackboard value to chase (true/false)
  (AI|Components|Blackboard|SetValueasBool (Variables|Default|GetBlackboard) (Utilities|Name|MakeLiteralName "CanChase") true))

(event EventStopChase
  ;[1 1 1] Start & Stop Chase Event - Set Blackboard value to chase (true/false)
  (Utilities|FlowControl|RetriggerableDelay 5.0)
  (AI|Components|Blackboard|SetValueasBool (Variables|Default|GetBlackboard) (Utilities|Name|MakeLiteralName "CanChase") false))

(fn ConstructionScript)

(fn HandleSightPerception
  (params (Actor :type Actor%20Object%20Reference) (Stimulus :type AI%20Stimulus%20Structure))
  (bind _self self)
  (bind _blackboard (Variables|Default|GetBlackboard))
  (bind _returnvalue (Class|AIPerceptionSystem|GetSenseClassforStimulus Stimulus))
  (if (and (== _returnvalue "/Script/AIModule.AISense_Sight") (.bSuccessfullySensed (Utilities|Struct|BreakAIStimulus Stimulus)))
    (AI|Components|Blackboard|SetValueasObject (Variables|Default|GetBlackboard) (Utilities|Name|MakeLiteralName "TargetActor") Actor)
    (Class|BPIAlertSystem|StartChase(Message) _self)
    (else
      (Class|BPIAlertSystem|StopChase(Message) _self)
      (if (not (ScalableFloat|GetValueasBool (Variables|Default|GetBlackboard) (Utilities|Name|MakeLiteralName "CanChase")))
        (AI|Components|Blackboard|SetValueasVector _blackboard (Utilities|Name|MakeLiteralName "TargetLocation") (Transformation|GetActorLocation Actor))
        (AI|Components|Blackboard|SetValueasObject _blackboard (Utilities|Name|MakeLiteralName "TargetActor") 0)))))

(fn HandleSoundPerception
  (params (Stimulus :type AI%20Stimulus%20Structure))
  (bind _returnvalue (Class|AIPerceptionSystem|GetSenseClassforStimulus Stimulus))
  (if (== _returnvalue "/Script/AIModule.AISense_Hearing")
    (AI|Components|Blackboard|SetValueasVector (Variables|Default|GetBlackboard) (Utilities|Name|MakeLiteralName "TargetLocation") (.StimulusLocation (Utilities|Struct|BreakAIStimulus Stimulus)))))