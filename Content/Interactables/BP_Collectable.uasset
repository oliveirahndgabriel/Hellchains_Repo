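; BP_Collectable is an interactable pickup that delivers health, key, power or lore items to the interacting actor.
; Interact switches on ItemType, calls the matching message on a valid actor (keys pass KeyNumber), then destroys itself after a short delay.
; DisplayButton reveals the interact widget and uses a retriggerable delay to hide it once calls stop, provided ShowButton is true.
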(event EventInteract
  (params (Actor :type Actor%20Object%20Reference))
  (bind _returnvalue (Utilities|IsValid Actor))
  (switch Utilities|FlowControl|Switch|SwitchonEN_CollectableType (Variables|Default|GetItem%20Type)
    (:NewEnumerator0
      (if _returnvalue
        (Class|BPIItems|AddHealth(Message) Actor)
        (Utilities|FlowControl|Delay 0.5 :!label _label)
        (Actor|DestroyActor)))
    (:NewEnumerator2
      (if _returnvalue
        (Class|BPIItems|AddKey(Message) Actor (Variables|Default|GetKeyNumber))
        (goto _label)))
    (:NewEnumerator1
      (if _returnvalue
        (Class|BPIItems|AddPower(Message) Actor)
        (goto _label)))
    (:NewEnumerator3
      (if _returnvalue
        (Class|BPIItems|AddLore(Message) Actor)
        (goto _label)))))

(event EventDisplayButton
  (params (ShowButton :type Boolean))
  ;[1 1 1] Interface Event - Display Interact Button
  (Rendering|SetVisibility (Variables|Default|GetWidget) true false)
  (Utilities|FlowControl|RetriggerableDelay 1.0)
  (if ShowButton
    (Rendering|SetVisibility (Variables|Default|GetWidget) false false)))

(fn ConstructionScript)