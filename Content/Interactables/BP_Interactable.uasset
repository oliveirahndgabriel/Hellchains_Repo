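; BP_Interactable is an interactable world actor that acts as either a readable note or a lever, chosen by its ENStates value.
; On Interact, a note opens the WD_TextNotes widget and pauses the game, while a lever calls ActivateMessage on the BP_Door found by class lookup.
; DisplayButton reveals its prompt widget, using a retriggerable delay to hide it after repeated calls stop, if ShowButton is true.
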(event EventInteract
  (params (Actor :type Actor%20Object%20Reference))
  (switch Utilities|FlowControl|Switch|SwitchonEN_InteractableStates (Variables|Default|GetEN_States)
    (:NewEnumerator0
      (bind _returnvalue (UserInterface|CreateWidget "/Game/Items/WD_TextNotes.WD_TextNotes_C"))
      (UserInterface|Viewport|AddtoViewport _returnvalue 0)
      (Game|SetGamePaused true))
    (:NewEnumerator1
      (bind _returnvalue_2 (Actor|GetActorOfClass "/Game/Interactables/BP_Door.BP_Door_C"))
      (Class|BPIInteract|Activate(Message) _returnvalue_2))))

(event EventDisplayButton
  (params (ShowButton :type Boolean))
  (Rendering|SetVisibility (Variables|Default|GetWidget) true false)
  (Utilities|FlowControl|RetriggerableDelay 1.0)
  (if ShowButton
    (Rendering|SetVisibility (Variables|Default|GetWidget) false false)))

(fn ConstructionScript)